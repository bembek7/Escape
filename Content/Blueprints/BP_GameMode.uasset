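; Game mode that builds a random chain of rooms from the starting room's exit and creates a default save if none exists.
; SpawnRooms recursively attaches rooms exit to exit, rerolling any that push net left or right turns too far, then caps the chain with BP_FinalRoom.
; Weighted picks redistribute the chosen room's weight to discourage repeats.
; Player death respawns and possesses a new pawn, clears rooms and grapple targets, and regenerates the level.
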(event `ClearRooms`
  (for _array_element (`self.CurrentRooms`)
    (`self.K2_DestroyActor` _array_element))
  (`KismetArrayLibrary.Array_Clear` (`self.CurrentRooms`))
  (bind _outactors (`GameplayStatics.GetAllActorsOfClass` "/Game/Blueprints/Interactive/BP_GrappleTarget.BP_GrappleTarget_C"))
  (for _array_element_2 _outactors
    (`self.K2_DestroyActor` _array_element_2)))

(event `Respawn`
  (`self.ClearRooms`)
  (bind _returnvalue (`GameplayStatics.GetActorOfClass` "/Game/Blueprints/Rooms/BP_Room.BP_Room_C" :!label _label))
  (`self.SpawnRooms` (`self.NumberOfRoomsToSpawn`) (`SceneComponent.K2_GetComponentToWorld` (`/Game/Blueprints/Rooms/BP_Room.BP_LevelExit` _returnvalue)))
  (bind _asbp_player (cast `/Game/Blueprints/BP_Player` (`GameplayStatics.GetPlayerCharacter` 0)))
  (set `self.Player` _asbp_player)
  (add `self.OnDestroyed` (`self.Player`) (delegate `OnPlayerDestroyed`)))

(event `self.ReceiveBeginPlay`
  (if (!= (`KismetArrayLibrary.Array_Length` (`self.ChancesOfSpawning`)) (`KismetArrayLibrary.Array_Length` (`self.RoomsClasses`)))
    (`KismetSystemLibrary.PrintString` "ARRAY OF CHANCES AND CLASSES ROOM ARE NOT THE SAME SIZE" true true (struct :`R` 1.0 :`B` 0.029831 :`A` 1.0)))
  (bind _returnvalue (`GameplayStatics.LoadGameFromSlot` "0"))
  (cast `/Game/Blueprints/BP_SaveGame` _returnvalue
    (:`then`
      _)
    (:`CastFailed`
      (bind _returnvalue_2 (`GameplayStatics.CreateSaveGameObject` "/Game/Blueprints/BP_SaveGame.BP_SaveGame_C"))
      (set `/Game/Blueprints/BP_SaveGame.PlayedTutorial` false _returnvalue_2)
      (`GameplayStatics.SaveGameToSlot` _returnvalue_2 "0")))
  (bind _asbp_player_controller (cast `/Game/Blueprints/BP_PlayerController` (`GameplayStatics.GetPlayerController` 0)))
  (set `self.PlayerController` _asbp_player_controller)
  (goto _label))

(event `OnPlayerDestroyed` :!signature `self.OnDestroyed`
  (params (DestroyedActor :type "Actor Object Reference"))
  (bind _returnvalue (`|SpawnActorFromClass` (`GameplayStatics.GetObjectClass` DestroyedActor) (`KismetMathLibrary.MakeTransform` (`/Game/Blueprints/BP_PlayerController.PlayerSpawnLocation` (`self.PlayerController`)) (struct :`Yaw` 90.0)) "Undefined" "OverrideRootScale" null null))
  (bind _asbp_player (cast `/Game/Blueprints/BP_Player` _returnvalue))
  (`Controller.Possess` (`GameplayStatics.GetPlayerController` 0) _asbp_player)
  (`/Game/Blueprints/BP_PlayerController.PlayerDied` (`self.PlayerController`))
  (`self.Respawn`))

(fn `GetRandomRoomIndex`
  (returns (RoomIndex :type Integer))
  (locals (AllRoomsArray :type "Array of Integer") (RandomizedIndex :type Integer) (ChancesOfChosenIndex :type Integer) (ChancesOfChosenPerSizeMinusOne :type Integer) (RestAfterDividing :type Integer))
  (bind _chancesofspawning (`self.ChancesOfSpawning`))
  (bind _output (`|GetArrayItem` _chancesofspawning (`KismetArrayLibrary.Array_LastIndex` _chancesofspawning)))
  ;[1 1 1] Randomizing
  (for (_array_element _array_index) (`self.ChancesOfSpawning`)
    (for _ (range 1 (+ _array_element 1))
      (`KismetArrayLibrary.Array_Add` (`local.AllRoomsArray`) _array_index)))
  (set `local.RandomizedIndex` (`KismetArrayLibrary.Array_Random` (`local.AllRoomsArray`)))
  ;[1 1 1] Updating the chances
  (set `local.ChancesOfChosenIndex` (`|GetArrayItem` (`self.ChancesOfSpawning`) (`local.RandomizedIndex`)))
  (set `local.ChancesOfChosenPerSizeMinusOne` (/ (`local.ChancesOfChosenIndex`) (- (`KismetArrayLibrary.Array_Length` (`self.ChancesOfSpawning`)) 1)))
  (set `local.RestAfterDividing` (mod (`local.ChancesOfChosenIndex`) (- (`KismetArrayLibrary.Array_Length` (`self.ChancesOfSpawning`)) 1)))
  (for (_array_element_2 _array_index_2) (`self.ChancesOfSpawning`)
    (if (!= _array_index_2 (`local.RandomizedIndex`))
      (`KismetArrayLibrary.Array_Set` _chancesofspawning _array_index_2 (+ _array_element_2 (`local.ChancesOfChosenPerSizeMinusOne`)))
      (else
        (`KismetArrayLibrary.Array_Set` _chancesofspawning _array_index_2))))
  (`|VariableSetRef` _output (+ _output (`local.RestAfterDividing`)))
  (return (`local.RandomizedIndex`)))

(fn `SpawnRooms`
  (params (RoomsToSpawn :type Integer) (OldExitTransform :type "Transform Structure"))
  (if (> RoomsToSpawn 0)
    (bind _roomindex (`self.GetRandomRoomIndex` :!label _label))
    (bind _output (`|GetArrayItem` (`self.RoomsClasses`) _roomindex))
    (bind (_busedexit _leftturn _rightturn) (defaults `Object` _output))
    (if (or (>= (+ (`self.LeftTurns`) _leftturn) 4) (>= (+ (`self.RightTurns`) _rightturn) 4))
      (goto _label)
      (else
        (bind _returnvalue (`|SpawnActorFromClass` _output (`KismetMathLibrary.MakeTransform` (.location OldExitTransform) (.rotation OldExitTransform)) "Undefined" "OverrideRootScale" null null))
        (`KismetArrayLibrary.Array_Add` (`self.CurrentRooms`) _returnvalue)
        (bind _leftturn_2 (`/Game/Blueprints/Rooms/BP_Room.LeftTurn` _returnvalue))
        (bind _rightturn_2 (`/Game/Blueprints/Rooms/BP_Room.RightTurn` _returnvalue))
        (set `self.LeftTurns` (- (+ (`self.LeftTurns`) _leftturn_2) _rightturn_2))
        (set `self.RightTurns` (- (+ (`self.RightTurns`) _rightturn_2) _leftturn_2))
        (bind _output_get (set `self.LastExitTransform` (`SceneComponent.K2_GetComponentToWorld` (`/Game/Blueprints/Rooms/BP_Room.BP_LevelExit` _returnvalue))))
        (`self.SpawnRooms` (- (`local.RoomsToSpawn`) 1) _output_get)))
    (else
      (bind _returnvalue_2 (`|SpawnActorFromClass` "/Game/Blueprints/Rooms/BP_FinalRoom.BP_FinalRoom_C" (`KismetMathLibrary.MakeTransform` (.location (`self.LastExitTransform`)) (.rotation (`self.LastExitTransform`))) "Undefined" "OverrideRootScale" null null))
      (`KismetArrayLibrary.Array_Add` (`self.CurrentRooms`) _returnvalue_2)
      (set `self.LastExitTransform` (`self.GetTransform` _returnvalue_2))
      (return))))

(fn `UserConstructionScript`)