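; Grapple line actor that draws a line between the player and a grapple target, with its end attached to a child of the player's capsule at BeginPlay.
; GrappleOn stores the target, shows the line and runs a fast looping timer for half a second that eases the line's origin toward the target with VInterpTo, using delta time cached on Tick.
; GrappleOff hides the line, leaving it at its current location.
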(event `self.ReceiveBeginPlay`
  (`CableComponent.SetAttachEndToComponent` (`self.GrappleLine`) (`SceneComponent.GetChildComponent` (`Character.CapsuleComponent` (`GameplayStatics.GetPlayerCharacter` 0)) 0) "None"))

(event `self.ReceiveTick`
  (params (DeltaSeconds :type "Float (single-precision)"))
  (set `self.Delta Seconds` DeltaSeconds))

(event `GrappleOff`
  (`SceneComponent.SetVisibility` (`self.GrappleLine`) false false)
  (`SceneComponent.K2_SetWorldLocation` (`self.GrappleLine`) (`SceneComponent.K2_GetComponentLocation` (`self.GrappleLine`)) false false))

(event `GrappleOn`
  (params (Target :type "Vector Structure"))
  (set `self.BeginningLocation` (`SceneComponent.K2_GetComponentLocation` (`self.GrappleLine`)))
  (set `self.GrappleTarget` Target)
  (`SceneComponent.SetVisibility` (`self.GrappleLine`) true false)
  (bind _returnvalue (`KismetSystemLibrary.K2_SetTimerDelegate` (delegate `CustomEvent_0`) 0.0001 true))
  (`KismetSystemLibrary.Delay` 0.5)
  (`KismetSystemLibrary.K2_ClearAndInvalidateTimerHandle` _returnvalue))

(event `CustomEvent_0`
  (`SceneComponent.K2_SetWorldLocation` (`self.GrappleLine`) (`KismetMathLibrary.VInterpTo` (`SceneComponent.K2_GetComponentLocation` (`self.GrappleLine`)) (`self.GrappleTarget`) (`self.Delta Seconds`) 0.04) false false))

(fn `UserConstructionScript`)