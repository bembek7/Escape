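; BP_Ladder is a ladder actor that switches the player's ladder state on BP_PlayerController as capsule components overlap its volumes.
; Entering Box passes the ladder's forward vector to EnteredLadder and blocks ToOut2 exits for a short delay.
; Leaving Box calls ExittedLadder, preceded by ExitBoost if the owner overlaps ToOut.
; Entering ToOut2 also calls ExittedLadder once CanOut is true.
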(event `self.ReceiveBeginPlay`
  (bind _asbp_player_controller (cast `/Game/Blueprints/BP_PlayerController` (`GameplayStatics.GetPlayerController` 0)))
  (set `self.PlayerController` _asbp_player_controller))

(event `self.Box.OnComponentBeginOverlap`
  (params (OverlappedComponent :type "PrimitiveComponent Object Reference") (OtherActor :type "Actor Object Reference") (OtherComp :type "PrimitiveComponent Object Reference") (OtherBodyIndex :type Integer) (bFromSweep :type Boolean) (SweepResult :type "HitResult Structure (by ref)"))
  (cast `CapsuleComponent` OtherComp)
  (`/Game/Blueprints/BP_PlayerController.EnteredLadder` (`self.PlayerController`) (`self.GetActorForwardVector`))
  (set `self.CanOut` false)
  (`KismetSystemLibrary.Delay` 0.2)
  (set `self.CanOut` true))

(event `self.Box.OnComponentEndOverlap`
  (params (OverlappedComponent :type "PrimitiveComponent Object Reference") (OtherActor :type "Actor Object Reference") (OtherComp :type "PrimitiveComponent Object Reference") (OtherBodyIndex :type Integer))
  (bind _playercontroller (`self.PlayerController`))
  (bind _ascapsule_collision (cast `CapsuleComponent` OtherComp))
  (if (`PrimitiveComponent.IsOverlappingActor` (`self.ToOut`) (`ActorComponent.GetOwner` _ascapsule_collision))
    (`/Game/Blueprints/BP_PlayerController.ExitBoost` _playercontroller))
  (`/Game/Blueprints/BP_PlayerController.ExittedLadder` _playercontroller))

(event `self.ToOut2.OnComponentBeginOverlap`
  (params (OverlappedComponent :type "PrimitiveComponent Object Reference") (OtherActor :type "Actor Object Reference") (OtherComp :type "PrimitiveComponent Object Reference") (OtherBodyIndex :type Integer) (bFromSweep :type Boolean) (SweepResult :type "HitResult Structure (by ref)"))
  (if (`self.CanOut`)
    (cast `CapsuleComponent` OtherComp)
    (`/Game/Blueprints/BP_PlayerController.ExittedLadder` (`self.PlayerController`))))

(fn `UserConstructionScript`)