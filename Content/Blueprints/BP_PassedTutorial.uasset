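; BP_PassedTutorial is a trigger volume actor that marks the tutorial as completed when the player reaches it.
; On BeginPlay it caches references to BP_PlayerController and BP_GameMode.
; When BP_Player overlaps its Box, it calls SetSavePlayedTutorial on the game mode with true and clears the controller's InTutorial flag.
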(event `self.ReceiveBeginPlay`
  (bind _asbp_player_controller (cast `/Game/Blueprints/BP_PlayerController` (`GameplayStatics.GetPlayerController` 0)))
  (set `self.PlayerController` _asbp_player_controller)
  (bind _asbp_game_mode (cast `/Game/Blueprints/BP_GameMode` (`GameplayStatics.GetGameMode`)))
  (set `self.GameMode` _asbp_game_mode))

(event `self.Box.OnComponentBeginOverlap`
  (params (OverlappedComponent :type "PrimitiveComponent Object Reference") (OtherActor :type "Actor Object Reference") (OtherComp :type "PrimitiveComponent Object Reference") (OtherBodyIndex :type Integer) (bFromSweep :type Boolean) (SweepResult :type "HitResult Structure (by ref)"))
  (cast `/Game/Blueprints/BP_Player` OtherActor)
  (`GMBase.SetSavePlayedTutorial` (`self.GameMode`) true)
  (set `PlayerControllerBase.bInTutorial` false (`self.PlayerController`)))

(fn `UserConstructionScript`)