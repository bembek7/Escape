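; Player controller for a first-person-style movement character, handling Enhanced Input for walk, look, jump, dash, crouch/slide, ladder climbing and wall running on BP_Player.
; Capsule hits on BP_WallToRunOn start wall runs, which a timeline sustains by line trace with zero gravity, plane constraint and camera roll.
; Slides begin above a speed threshold and decay into crouch via a timeline.
; Ladder events switch to flying movement, remapping input to vertical climbing.
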(event `BeginWallRun`
  (bind _charactermovement (`Character.CharacterMovement` (`self.PlayerChar`)))
  (bind _charactermovement_2 (`Character.CharacterMovement` (`self.PlayerChar`)))
  ;[1 0.4538 0.9554 1 30] Wall Run
  (set `self.Air Control` (`CharacterMovementComponent.AirControl` _charactermovement_2))
  (set `self.Gravity Scale` (`CharacterMovementComponent.GravityScale` _charactermovement_2))
  (set `CharacterMovementComponent.AirControl` 1.0 _charactermovement)
  (set `CharacterMovementComponent.GravityScale` 0.0 _charactermovement)
  (`MovementComponent.SetPlaneConstraintNormal` _charactermovement (0.0 0.0 1.0))
  (set `self.bIsWallRunning` true)
  (`self.BeginCameraTilt`)
  (`Timeline|WallRunTimeline` :!via `PlayFromStart` :!label _label
    (:`Update`
      (`self.UpdateWallRun`))))

(event `EnteredLadder`
  (params (LadderLocation :type "Vector Structure"))
  (bind _charactermovement (`Character.CharacterMovement` (`self.PlayerChar`)))
  (if (`self.bCanEnterLadder`)
    (set `self.bCanEnterLadder` false)
    (set `self.LadderForwardVector` LadderLocation)
    (set `self.bIsOnLadder` true)
    (`CharacterMovementComponent.SetMovementMode` _charactermovement "MOVE_Flying" 0)
    (set `MovementComponent.Velocity` (0.0 0.0 0.0) _charactermovement)))

(event `Dash`
  (if (`NavMovementComponent.IsFalling` (`Pawn.GetMovementComponent` (`self.PlayerChar`)))
    (set `self.DashForce` 2250.0)
    (else
      (set `self.DashForce` 2500.0)))
  (`Character.LaunchCharacter` (`self.PlayerChar`) (* (`KismetMathLibrary.Conv_RotatorToVector` (`Pawn.GetControlRotation` (`self.PlayerChar`))) (`self.DashForce`)) true true))

(event `ExittedLadder`
  (set `self.bIsOnLadder` false)
  (if (not (`self.bIsGrappling`))
    (`CharacterMovementComponent.SetMovementMode` (`Character.CharacterMovement` (`self.PlayerChar`)) "MOVE_Walking" 0))
  (`KismetSystemLibrary.Delay` 0.2)
  (set `self.bCanEnterLadder` true))

(event `self.ReceiveTick`
  (params (DeltaSeconds :type "Float (single-precision)")))

(event `EndWallRun`
  (bind _charactermovement (`Character.CharacterMovement` (`self.PlayerChar`)))
  ;[1 0.4538 0.9554 1 30] Wall Run
  (set `CharacterMovementComponent.AirControl` (`self.Air Control`) _charactermovement)
  (set `CharacterMovementComponent.GravityScale` (`self.Gravity Scale`) _charactermovement)
  (`MovementComponent.SetPlaneConstraintNormal` _charactermovement (0.0 0.0 0.0))
  (set `self.bIsWallRunning` false)
  (`self.EndCameraTilt`)
  (`|ExecutionSequence`
    (:`then_0`
      (goto _label :!via `Stop`))
    (:`then_1`
      (set `self.bWallRunReady` false)
      (`KismetSystemLibrary.K2_SetTimerDelegate` (delegate `CanWallRunAgain`) 0.2))))

(event `ExitBoost`
  (bind _playerchar (`self.PlayerChar`))
  (`Character.LaunchCharacter` _playerchar (* (`self.GetActorUpVector` _playerchar) 50.0) false false))

(event `CanWallRunAgain`
  ;[1 0.4538 0.9554 1 30] Wall Run
  (set `self.bWallRunReady` true))

(event `BeginCameraTilt`
  (bind (_returnvalue_roll _returnvalue_pitch _returnvalue_yaw) (`KismetMathLibrary.BreakRotator` (`self.GetControlRotation`)))
  ;[1 0.4538 0.9554 1 30] Wall Run
  (bind (_direction _cameradegrees) (`Timeline|CameraTiltTimeline` :!label _label_2)
    (:`Update`
      (`self.SetControlRotation` (`KismetMathLibrary.MakeRotator` (* _cameradegrees (select `/Game/Enums/E_WallRunSide` (`self.WallRunSide`) :`NewEnumerator0` -1.0 :`NewEnumerator1` 1.0)) _returnvalue_pitch _returnvalue_yaw)))))

(event `EndCameraTilt`
  ;[1 0.4538 0.9554 1 30] Wall Run
  (goto _label_2 :!via `Reverse`))

(event `self.ReceiveBeginPlay`
  (`EnhancedInputSubsystemInterface.AddMappingContext` (pcsubsystem `EnhancedInputLocalPlayerSubsystem` self) "/Game/Input/IMC_Player.IMC_Player" 0 (struct))
  (bind _asbp_player (cast `/Game/Blueprints/BP_Player` (`self.K2_GetPawn`)))
  (bind _output_get (set `self.PlayerChar` _asbp_player))
  (bind _charactermovement (`Character.CharacterMovement` _output_get))
  (set `self.WalkSpeed` (`CharacterMovementComponent.MaxWalkSpeed` _charactermovement))
  (set `self.DefaultCrouchSpeed` (`CharacterMovementComponent.MaxWalkSpeedCrouched` _charactermovement))
  ;[1 0.4538 0.9554 1 30] Wall Run
  (add `PrimitiveComponent.OnComponentHit` (`Character.CapsuleComponent` (`self.PlayerChar`)) (delegate `OnComponenentHitPlayerCapsule`)))

(event `OnComponenentHitPlayerCapsule`
  (params (HitComponent :type "PrimitiveComponent Object Reference") (OtherActor :type "Actor Object Reference") (OtherComp :type "PrimitiveComponent Object Reference") (NormalImpulse :type "Vector Structure") (Hit :type "HitResult Structure (by ref)"))
  (bind (_wallrunside _direction) (`self.FindRunDirectionAndSide` Hit_ImpactNormal))
  (bind _playerchar (`self.PlayerChar`))
  (bind _returnvalue_x (`KismetMathLibrary.BreakVector` (`KismetMathLibrary.LessLess_VectorRotator` (`self.GetVelocity` _playerchar) (`self.K2_GetActorRotation` _playerchar))))
  ;[1 0.4538 0.9554 1 30] Wall Run
  (cast `/Game/Blueprints/BP_WallToRunOn` OtherActor)
  (if (and (not (`self.bIsWallRunning`)) (`self.CanSurfaceBeWallRun` Hit_ImpactNormal) (`NavMovementComponent.IsFalling` (`Character.CharacterMovement` (`self.PlayerChar`))) (`self.bWallRunReady`) (> _returnvalue_x 100.0) (>= (`self.YAxis`) 0.0))
    (set `self.WallRunSide` _wallrunside)
    (set `self.WallRunDirection` _direction)
    (`self.BeginWallRun`)))

(event `EnhancedInput|/Game/Input/IA_Walk`
  (params (ActionValue :type "Vector2D Structure") (ElapsedSeconds :type "Float (double-precision)") (TriggeredSeconds :type "Float (double-precision)") (InputAction :type "InputAction Object Reference" :default "/Game/Input/IA_Walk.IA_Walk"))
  (bind _playerchar (`self.PlayerChar`))
  (bind _playerchar_2 (`self.PlayerChar`))
  (bind _playerchar_3 (`self.PlayerChar`))
  (bind _playerchar_4 (`self.PlayerChar`))
  (bind _playerchar_5 (`self.PlayerChar`))
  (bind _playerchar_6 (`self.PlayerChar`))
  ;[1 0.4583 0.6625 1 30] Input
  (:`Triggered`
    (set `self.YAxis` ActionValue_Y)
    (if (not (`self.bIsOnLadder`))
      (`Pawn.AddMovementInput` _playerchar_2 (`SceneComponent.GetRightVector` (`Actor.RootComponent` _playerchar_2)) ActionValue_X false)
      (`Pawn.AddMovementInput` _playerchar (`SceneComponent.GetForwardVector` (`Actor.RootComponent` _playerchar)) ActionValue_Y false)
      (else
        (`|ExecutionSequence`
          (:`then_0`
            (if (!= ActionValue_X 0.0)
              (if (< (`KismetMathLibrary.Dot_VectorVector` (`self.LadderForwardVector`) (* (`self.GetActorRightVector` (`self.PlayerChar`)) ActionValue_X)) 0.0)
                (`Pawn.AddMovementInput` _playerchar_6 (`self.GetActorUpVector` _playerchar_6) 1.0 false)
                (else
                  (`Pawn.AddMovementInput` _playerchar_3 (`self.GetActorUpVector` _playerchar_3) -1.0 false)))))
          (:`then_1`
            (if (!= ActionValue_Y 0.0)
              (if (< (`KismetMathLibrary.Dot_VectorVector` (`self.LadderForwardVector`) (* (`self.GetActorForwardVector` (`self.PlayerChar`)) ActionValue_Y)) 0.0)
                (`Pawn.AddMovementInput` _playerchar_4 (`self.GetActorUpVector` _playerchar_4) 1.0 false)
                (else
                  (`Pawn.AddMovementInput` _playerchar_5 (`self.GetActorUpVector` _playerchar_5) -1.0 false))))))))))

(event `EnhancedInput|/Game/Input/IA_Jump`
  (params (ActionValue :type Boolean) (ElapsedSeconds :type "Float (double-precision)") (TriggeredSeconds :type "Float (double-precision)") (InputAction :type "InputAction Object Reference" :default "/Game/Input/IA_Jump.IA_Jump"))
  (bind _playerchar (`self.PlayerChar`))
  ;[1 0.4583 0.6625 1 30] Input
  (:`Triggered`
    (`Character.Jump` (`self.PlayerChar`))
    (if (`self.bIsOnLadder`)
      (`Character.LaunchCharacter` (`self.PlayerChar`) (* (`self.LadderForwardVector`) 1000.0) false false)
      (elif (`self.bIsWallRunning`)
        (`Character.LaunchCharacter` _playerchar (`self.FindLaunchVelocity`) false false)
        (`self.EndWallRun`)
        (else
          (`Character.Jump` _playerchar))))))

(event `NormalCrouch`
  ;[1 0.4583 0.6625 1 30] Input
  (set `self.bIsCrouching` true)
  (set `self.bIsSliding` false)
  (set `CharacterMovementComponent.MaxWalkSpeedCrouched` (`self.DefaultCrouchSpeed`) (`Character.CharacterMovement` (`self.PlayerChar`)))
  (`Character.Crouch` (`self.PlayerChar`)))

(event `EnhancedInput|/Game/Input/IA_CrouchSlide`
  (params (ActionValue :type Boolean) (ElapsedSeconds :type "Float (double-precision)") (TriggeredSeconds :type "Float (double-precision)") (InputAction :type "InputAction Object Reference" :default "/Game/Input/IA_CrouchSlide.IA_CrouchSlide"))
  (bind _charactermovement (`Character.CharacterMovement` (`self.PlayerChar`)))
  (bind _charactermovement_2 (`Character.CharacterMovement` (`self.PlayerChar`)))
  (bind _velocity (`MovementComponent.Velocity` _charactermovement_2))
  (bind _maxwalkspeedcrouched (`CharacterMovementComponent.MaxWalkSpeedCrouched` _charactermovement))
  (bind _returnvalue (+ (`KismetMathLibrary.VSizeXY` (`MovementComponent.Velocity` (`Character.CharacterMovement` (`self.PlayerChar`)))) (`self.SlideAdditionalSpeed`)))
  ;[1 0.4583 0.6625 1 30] Input
  (:`Triggered`
    (`/Engine/EditorBlueprintResources/StandardMacros.DoOnce` false :!label _label_3
      (:`Completed`
        (if (not (or (`self.bIsCrouching`) (`self.bIsSliding`)))
          (if (`NavMovementComponent.IsMovingOnGround` _charactermovement_2) :!label _label_4
            (if (>= (`KismetMathLibrary.VSizeXY` _velocity) (`self.SpeedNeededToSlide`))
              (set `self.bIsSliding` true)
              (`Character.Crouch` (`self.PlayerChar`))
              (bind _output_get (set `CharacterMovementComponent.MaxWalkSpeedCrouched` _returnvalue (`Character.CharacterMovement` (`self.PlayerChar`))))
              (set `self.SlideSpeedDifference` (- _output_get (`self.DefaultCrouchSpeed`)))
              (`CharacterMovementComponent.AddImpulse` (`Character.CharacterMovement` (`self.PlayerChar`)) (* (`KismetMathLibrary.Normal` _velocity) _returnvalue) false)
              (bind (_direction _speed) (`Timeline|SlowingSlide` :!via `PlayFromStart` :!label _label_5)
                (:`Update`
                  (bind _output_get_2 (set `CharacterMovementComponent.MaxWalkSpeedCrouched` (- _maxwalkspeedcrouched (* _speed (`self.SlideSpeedDifference`))) _charactermovement))
                  (set `self.SlideSpeedDifference` (- _maxwalkspeedcrouched (`self.DefaultCrouchSpeed`)))
                  (if (`NavMovementComponent.IsCrouching` (`Character.CharacterMovement` (`self.PlayerChar`)))
                    (if (<= _output_get_2 (+ (`self.DefaultCrouchSpeed`) 50.0))
                      (`self.NormalCrouch`)
                      (goto _label_5 :!via `Stop`))
                    (else
                      (goto _label_5 :!via `Stop`)))))
              (else
                (`self.NormalCrouch`)))
            (else
              (goto _label_3 :!via `Reset`)))))))
  (:`Started`
    (goto _label_4))
  (:`Completed`
    (set `self.bIsCrouching` false)
    (set `self.bIsSliding` false)
    (set `CharacterMovementComponent.MaxWalkSpeedCrouched` (`self.DefaultCrouchSpeed`) (`Character.CharacterMovement` (`self.PlayerChar`)))
    (`Character.UnCrouch` (`self.PlayerChar`))))

(event `EnhancedInput|/Game/Input/IA_Look`
  (params (ActionValue :type "Vector2D Structure") (ElapsedSeconds :type "Float (double-precision)") (TriggeredSeconds :type "Float (double-precision)") (InputAction :type "InputAction Object Reference" :default "/Game/Input/IA_Look.IA_Look"))
  (bind _playerchar (`self.PlayerChar`))
  ;[1 0.4583 0.6625 1 30] Input
  (:`Triggered`
    (`Pawn.AddControllerYawInput` _playerchar (* ActionValue_X (`self.MouseXSensitivity`)))
    (`Pawn.AddControllerPitchInput` _playerchar (* ActionValue_Y -1.0 (`self.MouseYSensitivity`)))))

(event `EnhancedInput|/Game/Input/IA_Dash`
  (params (ActionValue :type Boolean) (ElapsedSeconds :type "Float (double-precision)") (TriggeredSeconds :type "Float (double-precision)") (InputAction :type "InputAction Object Reference" :default "/Game/Input/IA_Dash.IA_Dash"))
  ;[1 0.4583 0.6625 1 30] Input
  (:`Triggered`
    (`self.Dash`)))

(fn `CanSurfaceBeWallRun`
  (params (SurfaceNormal :type "Vector Structure"))
  (returns (ReturnValue :type Boolean))
  (return (and (not (< (.z SurfaceNormal) -0.05)) (< (`KismetMathLibrary.DegAcos` (`KismetMathLibrary.Dot_VectorVector` (`KismetMathLibrary.Normal` (`KismetMathLibrary.MakeVector` (.x SurfaceNormal) (.y SurfaceNormal))) SurfaceNormal)) (`CharacterMovementComponent.K2_GetWalkableFloorAngle` (`Character.CharacterMovement` (`self.PlayerChar`)))))))

(fn `FindLaunchVelocity`
  (returns (LaunchVelocity :type "Vector Structure"))
  (if (`self.bIsWallRunning`)
    (return (/ (* (+ (`KismetMathLibrary.Cross_VectorVector` (`self.WallRunDirection`) (select `byte` (`self.WallRunSide`) :`0` (0.0 0.0 1.0) :`1` (0.0 0.0 -1.0) :!type "Vector Structure")) (0.0 0.0 1.0)) (`CharacterMovementComponent.JumpZVelocity` (`Character.CharacterMovement` (`self.PlayerChar`)))) 2))))

(fn `FindRunDirectionAndSide`
  (params (`Wall Normal` :type "Vector Structure"))
  (returns (WallRunSide :type "/Game/Enums/E_WallRunSide Enum") (Direction :type "Vector Structure"))
  (locals (`Side(Local)` :type "/Game/Enums/E_WallRunSide Enum"))
  (bind _output_get (set `local.Side(Local)` (select `bool` (> (`KismetMathLibrary.DotProduct2D` (`KismetMathLibrary.Conv_VectorToVector2D` `Wall Normal`) (`KismetMathLibrary.Conv_VectorToVector2D` (`self.GetActorRightVector` (`self.PlayerChar`)))) 0.0) :`false` "NewEnumerator0" :`true` "NewEnumerator1" :!type "/Game/Enums/E_WallRunSide Enum")))
  (return _output_get (`KismetMathLibrary.Cross_VectorVector` (`local.Wall Normal`) (select `byte` _output_get :`0` (0.0 0.0 -1.0) :`1` (0.0 0.0 1.0) :!type "Vector Structure"))))

(fn `UpdateWallRun`
  (bind _returnvalue (`self.K2_GetActorLocation` (`self.PlayerChar`)))
  (bind (_outhit _returnvalue_2) (`KismetSystemLibrary.LineTraceSingle` _returnvalue (+ _returnvalue (* (`KismetMathLibrary.Cross_VectorVector` (`self.WallRunDirection`) (select `byte` (`self.WallRunSide`) :`0` (0.0 0.0 -1.0) :`1` (0.0 0.0 1.0) :!type "Vector Structure")) 200.0)) "TraceTypeQuery1"))
  (if _returnvalue_2
    (cast `/Game/Blueprints/BP_WallToRunOn` (`.HitActor` (`GameplayStatics.BreakHitResult` _outhit))
      (:`then`
        (bind (_wallrunside _direction) (`self.FindRunDirectionAndSide` (`.ImpactNormal` (`GameplayStatics.BreakHitResult` _outhit))))
        (if (`|EnumEquality` _wallrunside (`self.WallRunSide`))
          (bind _output_get (set `self.WallRunDirection` _direction))
          (bind (_returnvalue_x _returnvalue_y) (`KismetMathLibrary.BreakVector` (* _output_get (`MovementComponent.GetMaxSpeed` (`Character.CharacterMovement` (`self.PlayerChar`))))))
          (set `MovementComponent.Velocity` (`KismetMathLibrary.MakeVector` _returnvalue_x _returnvalue_y) (`Character.CharacterMovement` (`self.PlayerChar`)))
          (else
            (`self.EndWallRun`))))
      (:`CastFailed`
        (`self.EndWallRun` :!label _label)))
    (else
      (goto _label))))

(fn `UserConstructionScript`)