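; Interactive ladder actor that switches the player's PlayerBase character into and out of ladder movement through trigger volumes.
; Box overlap by any capsule signals player 0 to enter with the ladder's forward vector, and leaving it signals exit.
; Leaving Box while inside ToOut adds an exit boost.
; ToOut2 also forces an exit, blocked by CanOut for a brief delay after entry to avoid immediate dismounts.
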(event `self.ReceiveBeginPlay`)

(event `self.Box.OnComponentBeginOverlap`
  (params (OverlappedComponent :type "PrimitiveComponent Object Reference") (OtherActor :type "Actor Object Reference") (OtherComp :type "PrimitiveComponent Object Reference") (OtherBodyIndex :type Integer) (bFromSweep :type Boolean) (SweepResult :type "HitResult Structure (by ref)"))
  (cast `CapsuleComponent` OtherComp)
  (bind _asplayer_base (cast `PlayerBase` (`GameplayStatics.GetPlayerCharacter` 0)))
  (`PlayerBase.EnteredLadder` _asplayer_base (`self.GetActorForwardVector`))
  (set `self.CanOut` false)
  (`KismetSystemLibrary.Delay` 0.2)
  (set `self.CanOut` true))

(event `self.Box.OnComponentEndOverlap`
  (params (OverlappedComponent :type "PrimitiveComponent Object Reference") (OtherActor :type "Actor Object Reference") (OtherComp :type "PrimitiveComponent Object Reference") (OtherBodyIndex :type Integer))
  (bind _ascapsule_collision (cast `CapsuleComponent` OtherComp))
  (bind _asplayer_base (cast `PlayerBase` (`GameplayStatics.GetPlayerCharacter` 0)))
  (if (`PrimitiveComponent.IsOverlappingActor` (`self.ToOut`) (`ActorComponent.GetOwner` _ascapsule_collision))
    (`PlayerBase.ExitLadderBoost` _asplayer_base))
  (`PlayerBase.ExittedLadder` _asplayer_base))

(event `self.ToOut2.OnComponentBeginOverlap`
  (params (OverlappedComponent :type "PrimitiveComponent Object Reference") (OtherActor :type "Actor Object Reference") (OtherComp :type "PrimitiveComponent Object Reference") (OtherBodyIndex :type Integer) (bFromSweep :type Boolean) (SweepResult :type "HitResult Structure (by ref)"))
  (if (`self.CanOut`)
    (bind _asplayer_base (cast `PlayerBase` OtherActor))
    (`PlayerBase.ExittedLadder` _asplayer_base)))

(fn `UserConstructionScript`)